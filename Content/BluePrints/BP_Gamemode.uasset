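; BP_Gamemode is a game mode Blueprint that keeps the player's running score.
; At BeginPlay it binds SetSpeed to a changed-speed event, so it tracks the current Speed value.
; Each tick while the game is not paused, it adds Speed times delta seconds to Score, making score grow with distance travelled.
; GameStart resets Score to zero.
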(event Custom|SetSpeed
  (params (speed :type Float%20%28double-precision%29))
  (Variables|Default|SetSpeed speed))

(event EventBeginPlay
  (EventDispatchers|BindEventtoChangedSpeed (delegate Custom|SetSpeed)))

(event EventTick
  (params (DeltaSeconds :type Float%20%28single-precision%29))
  (if (not (Game|IsGamePaused))
    (Variables|Default|SetScore (+ (* DeltaSeconds (Variables|Default|GetSpeed)) (Variables|Default|GetScore)))))

(fn ConstructionScript)

(fn GameStart
  (Variables|Default|SetScore 0.0))