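; Enemy thunderbolt attack actor that telegraphs an area with a decal, then strikes it with lightning to damage the player.
; While visible, Tick grows the decal material's NowRadius toward its MaxRadius over BeforeDelayTime.
; A DoOnce then spawns and attaches BP_ky_lightning3 and enables DamageArea overlaps, which call GetDamaged on BP_MyPlayer.
; After AfterDelayTime it calls SetActive(false), disables overlaps and resets the timer and DoOnce for reuse.
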(event OnComponentBeginOverlap(damageArea)
  (params (OverlappedComponent :type Primitive%20Component%20Object%20Reference) (OtherActor :type Actor%20Object%20Reference) (OtherComp :type Primitive%20Component%20Object%20Reference) (OtherBodyIndex :type Integer) (bFromSweep :type Boolean) (SweepResult :type Hit%20Result%20Structure%20%28by%20ref%29))
  (bind _asbp_my_player (Utilities|Casting|CastToBP_MyPlayer OtherActor))
  (Class|MyPlayer|GetDamaged _asbp_my_player (Variables|Default|Getdamage)))

(event OnComponentEndOverlap(damageArea)
  (params (OverlappedComponent :type Primitive%20Component%20Object%20Reference) (OtherActor :type Actor%20Object%20Reference) (OtherComp :type Primitive%20Component%20Object%20Reference) (OtherBodyIndex :type Integer)))

(event EventBeginPlay
  (Variables|Default|SetnowTime 0.0)
  (bind _returnvalue (Rendering|Material|CreateDynamicMaterialInstance (Variables|Default|GetDecal) :!class /Script/Engine.DecalComponent))
  (bind _output_get (Variables|Default|SetAreaMaterialInstance _returnvalue))
  (bind _returnvalue_2 (Rendering|Material|GetScalarParameterValue _output_get "MaxRadius" :!class /Script/Engine.MaterialInstanceDynamic))
  (Variables|Default|SetMaxTime _returnvalue_2))

(event Collision|EventActorBeginOverlap
  (params (OtherActor :type Actor%20Object%20Reference)))

(event EventTick
  (params (DeltaSeconds :type Float%20%28single-precision%29))
  (bind _beforedelaytime (Variables|Default|GetbeforeDelayTime))
  (bind _particlepoint (Variables|Default|GetParticlePoint))
  (bind _relativelocation (Variables|/Script/Engine.SceneComponent|GetRelativeLocation _particlepoint))
  (if (not (Variables|Default|GetbHidden))
    (bind _output_get (Variables|Default|SetnowTime (+ DeltaSeconds (Variables|Default|GetnowTime))))
    (if (< _output_get _beforedelaytime)
      (Rendering|Material|SetScalarParameterValue (Variables|Default|GetAreaMaterialInstance) "NowRadius" (* (/ _output_get _beforedelaytime) (Variables|Default|GetMaxTime)) :!class /Script/Engine.MaterialInstanceDynamic)
      (else
        (Utilities|FlowControl|DoOnce false :!label _label
          (:Completed
            (bind _returnvalue (Game|SpawnActorfromClass "/Game/FXVarietyPack/Blueprints/BP_ky_lightning3.BP_ky_lightning3_C" (Math|Transform|MakeTransform (Math|Vector|MakeVector (- (.x _relativelocation) 5e+01) (.y _relativelocation) (.z _relativelocation)) "0, 0, 0" "0.200000,0.200000,0.200000") "Undefined" "MultiplyWithRoot" 0 0))
            (Transformation|AttachActorToActor _returnvalue self "None" "KeepRelative" "KeepRelative" "KeepRelative" true)
            (Variables|/Script/Engine.PrimitiveComponent|SetbGenerateOverlapEvents (Variables|Default|GetdamageArea) true)
            (Utilities|FlowControl|Delay (Variables|Default|GetafterDelayTime))
            (Class|ObjectPoolActor|SetActive false)
            (Variables|/Script/Engine.PrimitiveComponent|SetbGenerateOverlapEvents (Variables|Default|GetdamageArea) false)
            (Variables|Default|SetnowTime 0.0)
            (goto _label Reset)))))))

(fn ConstructionScript)