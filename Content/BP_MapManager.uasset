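; BP_MapManager tracks map speed and player-damaged state, linking both to BP_Gamemode.
; On BeginPlay it binds to the gamemode's damage start and end events, which toggle the damaged flag through SetPlayerDamaged.
; CalTotalSpeed extends the parent's calculation, then broadcasts TotalSpeed through the gamemode's CallChangedSpeed.
; An initial speed calculation runs after a short startup delay.
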(event Custom|PlayerDamagedStart
  ;[1 1 1] Player 피격 시 실행 함수(Bind)
  (Class|MapManager|SetPlayerDamaged true))

(event Custom|PlayerDamagedEnd
  ;[1 1 1] Player 피격 시 실행 함수(Bind)
  (Class|MapManager|SetPlayerDamaged false))

(event EventBeginPlay
  (bind _output_get (Variables|Default|SetGamemode (.AsBP%20Gamemode (Utilities|Casting|CastToBP_Gamemode (Game|GetGameMode)))))
  (EventDispatchers|BindEventtoPlayerDamagedStart _output_get (EventDispatchers|CreateEvent :!event Custom|PlayerDamagedStart))
  (EventDispatchers|BindEventtoPlayerDamagedEnd _output_get (EventDispatchers|CreateEvent :!event Custom|PlayerDamagedEnd))
  (Utilities|FlowControl|Delay 0.1)
  (Class|MapManager|CalTotalSpeed))

(event Collision|EventActorBeginOverlap
  (params (OtherActor :type Actor%20Object%20Reference)))

(event EventTick
  (params (DeltaSeconds :type Float%20%28single-precision%29)))

(event EventCalTotalSpeed
  ;[1 1 1] Speed 변경 시 호출(Call)
  (|CallParentFunction)
  (Default|CallChangedSpeed (Variables|Default|GetGamemode) (Variables|Default|GettotalSpeed)))

(fn ConstructionScript)